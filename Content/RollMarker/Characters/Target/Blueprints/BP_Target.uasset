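; BP_Target is a wandering AI target that gets marked red or cleaned yellow on contact in a marking game.
; Tick, through a random delay, sends it to random reachable points nearby.
; On overlap, the player marks it, a cleaner cleans it or spreads a mark depending on its own state, and marked targets infect clean ones.
; Clean state is read from the mesh material, and each change notifies BP_WinCondition and plays a sound.
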(event `self.ReceiveTick`
  (params (DeltaSeconds :type "Float (single-precision)"))
  ;[1 1 1] AI Movement (1 5
  (`KismetSystemLibrary.Delay` (`KismetMathLibrary.RandomFloatInRange` 1.0 5.0))
  (`|AIMoveTo` self (`NavigationSystemV1.K2_GetRandomReachablePointInRadius` (`self.K2_GetActorLocation`) 1000.0 null null) null))

(event `self.ReceiveActorBeginOverlap`
  (params (OtherActor :type "Actor Object Reference"))
  ;[1 1 1] Marking
  (bind _asbp_third_person_character (cast `/Game/RollMarker/Characters/Player/Blueprints/ThirdPerson/Blueprints/BP_ThirdPersonCharacter` OtherActor)
    (:`then`
      (bind _istargetclean (`self.DoTargetClean`))
      (`self.HitPlayerToTarget` _istargetclean _asbp_third_person_character))
    (:`CastFailed`
      (bind _asbp_cleaner (cast `/Game/RollMarker/Characters/Cleaner/Blueprints/BP_Cleaner` OtherActor)
        (:`then`
          (bind _iscleanerclean (`/Game/RollMarker/Characters/Cleaner/Blueprints/BP_Cleaner.DoCleanerClean` _asbp_cleaner))
          (bind _istargetclean_2 (`self.DoTargetClean`))
          (`self.HitCleanerToTarget` _istargetclean_2 _iscleanerclean))
        (:`CastFailed`
          (bind _asbp_target (cast `/Game/RollMarker/Characters/Target/Blueprints/BP_Target` OtherActor))
          (bind _istargetclean_3 (`self.DoTargetClean` _asbp_target))
          (bind _istargetclean_4 (`self.DoTargetClean`))
          (`self.HitTargetToTarget` _istargetclean_4 _istargetclean_3 _asbp_target))))))

(fn `DoTargetClean`
  (returns (isTargetClean :type Boolean))
  (if (== "/Game/RollMarker/Characters/Target/Materials/M_Yellow_Inst.M_Yellow_Inst" (`PrimitiveComponent.GetMaterial` (`self.MeshComponent`) 0))
    (return true)
    (else
      (return false))))

(fn `HitCleanerToTarget`
  (params (isTargetClean :type Boolean) (isCleanerClean :type Boolean))
  (bind _meshcomponent (`self.MeshComponent`))
  (if isCleanerClean
    (if (not isTargetClean)
      (`PrimitiveComponent.SetMaterial` _meshcomponent 0 "/Game/RollMarker/Characters/Target/Materials/M_Yellow_Inst.M_Yellow_Inst")
      (bind _outactors (`GameplayStatics.GetAllActorsOfClass` "/Game/RollMarker/Blueprints/BP_WinCondition.BP_WinCondition_C"))
      (`/Game/RollMarker/Blueprints/BP_WinCondition.CheckMarked` _outactors false)
      (`GameplayStatics.PlaySound2D` (`self.CleanedSound`) 0.2 1.0 0.0 null null))
    (elif isTargetClean
      (`PrimitiveComponent.SetMaterial` _meshcomponent 0 "/Game/RollMarker/Characters/Player/Materials/M_Red_Inst.M_Red_Inst")
      (bind _outactors_2 (`GameplayStatics.GetAllActorsOfClass` "/Game/RollMarker/Blueprints/BP_WinCondition.BP_WinCondition_C"))
      (`/Game/RollMarker/Blueprints/BP_WinCondition.CheckMarked` _outactors_2 true)
      (`GameplayStatics.PlaySound2D` (`self.MarkedSound`) 0.2 1.0 0.1 null null))))

(fn `HitPlayerToTarget`
  (params (IsTargetClean :type Boolean) (PlayerRef :type "/Game/RollMarker/Characters/Player/Blueprints/ThirdPerson/Blueprints/BP_ThirdPersonCharacter Object Reference"))
  (if IsTargetClean
    (`PrimitiveComponent.SetMaterial` (`self.MeshComponent`) 0 "/Game/RollMarker/Characters/Player/Materials/M_Red_Inst.M_Red_Inst")
    (bind _outactors (`GameplayStatics.GetAllActorsOfClass` "/Game/RollMarker/Blueprints/BP_WinCondition.BP_WinCondition_C"))
    (`/Game/RollMarker/Blueprints/BP_WinCondition.CheckMarked` _outactors true)
    (`GameplayStatics.PlaySound2D` (`self.MarkedSound`) 0.5 0.7 0.0 null null)))

(fn `HitTargetToTarget`
  (params (isTargetClean :type Boolean) (isCollidedTargetClean :type Boolean) (TargetRef :type "/Game/RollMarker/Characters/Target/Blueprints/BP_Target Object Reference"))
  (if isTargetClean
    (if (not isCollidedTargetClean)
      (`PrimitiveComponent.SetMaterial` (`self.MeshComponent`) 0 "/Game/RollMarker/Characters/Player/Materials/M_Red_Inst.M_Red_Inst")
      (bind _outactors (`GameplayStatics.GetAllActorsOfClass` "/Game/RollMarker/Blueprints/BP_WinCondition.BP_WinCondition_C" :!label _label))
      (`/Game/RollMarker/Blueprints/BP_WinCondition.CheckMarked` _outactors true)
      (`GameplayStatics.PlaySound2D` (`self.MarkedSound`) 0.2 1.0 0.1 null null))
    (elif isCollidedTargetClean
      (`PrimitiveComponent.SetMaterial` (`DefaultPawn.MeshComponent` TargetRef) 0 "/Game/RollMarker/Characters/Player/Materials/M_Red_Inst.M_Red_Inst")
      (goto _label))))

(fn `UserConstructionScript`)