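; BP_Cleaner is an AI pawn that wanders to random reachable points and, while clean and allowed to chase, pursues marked BP_Target pawns it sees.
; The player's touch marks a clean Cleaner red, and contact between clean and marked Cleaners turns the marked one green.
; Clean state is read directly from the mesh material, and each change calls CheckMarked on BP_WinCondition and plays a sound.
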(event `self.PawnSensing.OnSeePawn`
  (params (Pawn :type "Pawn Object Reference"))
  ;[1 1 1] AI chasing (Cleaner targets marked Target cubes)
  (if (`self.IsChaseTarget`)
    (bind _iscleanerclean (`self.DoCleanerClean`))
    (if _iscleanerclean
      (bind _asbp_target (cast `/Game/RollMarker/Characters/Target/Blueprints/BP_Target` Pawn))
      (bind _istargetclean (`/Game/RollMarker/Characters/Target/Blueprints/BP_Target.DoTargetClean` _asbp_target))
      (if (not _istargetclean)
        (`|AIMoveTo` self (0.0 0.0 0.0) _asbp_target)))))

(event `self.ReceiveTick`
  (params (DeltaSeconds :type "Float (single-precision)"))
  ;[1 1 1] AI Movement
  (`KismetSystemLibrary.Delay` (`KismetMathLibrary.RandomFloatInRange` 2.0 7.0))
  (`|AIMoveTo` self (`NavigationSystemV1.K2_GetRandomReachablePointInRadius` (`self.K2_GetActorLocation`) 1000.0 null null) null))

(event `self.ReceiveActorBeginOverlap`
  (params (OtherActor :type "Actor Object Reference"))
  ;[1 1 1] Marking
  (cast `/Game/RollMarker/Characters/Player/Blueprints/ThirdPerson/Blueprints/BP_ThirdPersonCharacter` OtherActor
    (:`then`
      (bind _iscleanerclean (`self.DoCleanerClean`))
      (`self.HitPlayerToCleaner` _iscleanerclean))
    (:`CastFailed`
      (bind _asbp_cleaner (cast `/Game/RollMarker/Characters/Cleaner/Blueprints/BP_Cleaner` OtherActor))
      (bind _iscleanerclean_2 (`self.DoCleanerClean` _asbp_cleaner))
      (bind _iscleanerclean_3 (`self.DoCleanerClean`))
      (`self.HitCleanerToCleaner` _iscleanerclean_3 _iscleanerclean_2 _asbp_cleaner))))

(fn `DoCleanerClean`
  (returns (isCleanerClean :type Boolean))
  (if (== "/Game/RollMarker/Characters/Cleaner/Materials/M_Green_Inst.M_Green_Inst" (`PrimitiveComponent.GetMaterial` (`self.MeshComponent`) 0))
    (return true)
    (else
      (return false))))

(fn `HitCleanerToCleaner`
  (params (isCleanerClean :type Boolean) (isCollidedCleanerClean :type Boolean) (CleanerRef :type "/Game/RollMarker/Characters/Cleaner/Blueprints/BP_Cleaner Object Reference"))
  (if isCollidedCleanerClean
    (if (not isCleanerClean)
      (`PrimitiveComponent.SetMaterial` (`self.MeshComponent`) 0 "/Game/RollMarker/Characters/Cleaner/Materials/M_Green_Inst.M_Green_Inst")
      (bind _outactors (`GameplayStatics.GetAllActorsOfClass` "/Game/RollMarker/Blueprints/BP_WinCondition.BP_WinCondition_C" :!label _label))
      (`/Game/RollMarker/Blueprints/BP_WinCondition.CheckMarked` _outactors false)
      (`GameplayStatics.PlaySound2D` (`self.CleanedSound`) 0.2 1.0 0.0 null null))
    (elif isCleanerClean
      (`PrimitiveComponent.SetMaterial` (`DefaultPawn.MeshComponent` CleanerRef) 0 "/Game/RollMarker/Characters/Cleaner/Materials/M_Green_Inst.M_Green_Inst")
      (goto _label))))

(fn `HitPlayerToCleaner`
  (params (isCleanerClean :type Boolean))
  (if isCleanerClean
    (`PrimitiveComponent.SetMaterial` (`self.MeshComponent`) 0 "/Game/RollMarker/Characters/Player/Materials/M_Red_Inst.M_Red_Inst")
    (bind _outactors (`GameplayStatics.GetAllActorsOfClass` "/Game/RollMarker/Blueprints/BP_WinCondition.BP_WinCondition_C"))
    (`/Game/RollMarker/Blueprints/BP_WinCondition.CheckMarked` _outactors true)
    (`GameplayStatics.PlaySound2D` (`self.MarkedSound`) 0.2 0.8 0.0 null null)))

(fn `UserConstructionScript`)