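; BP_WinCondition tracks marked cubes in RollMarker and triggers victory when every cube is marked.
; On BeginPlay it finds BP_Brain and BP_ScoreBoard, then Tick waits for the Brain's counted flag to cache the total once and refresh the scoreboard.
; CheckMarked adjusts the marked count and pushes it to both.
; When counts match, a one-shot Victory plays a sound, shows W_VictoryScreen, pauses and switches to UI-only input.
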(event `GetScoreboardRef`
  ;[1 1 1] References
  (bind _outactors (`GameplayStatics.GetAllActorsOfClass` "/Game/RollMarker/Blueprints/BP_ScoreBoard.BP_ScoreBoard_C"))
  (set `self.ScoreboardRef` (`|GetArrayItem` _outactors)))

(event `GetBrainRef`
  ;[1 1 1] References
  (bind _outactors (`GameplayStatics.GetAllActorsOfClass` "/Game/RollMarker/Blueprints/BP_Brain.BP_Brain_C"))
  (set `self.BrainRef` (`|GetArrayItem` _outactors)))

(event `self.ReceiveBeginPlay`
  ;[1 1 1] Begin
  (`self.GetBrainRef`)
  (`self.GetScoreboardRef`))

(event `self.ReceiveTick`
  (params (DeltaSeconds :type "Float (single-precision)"))
  ;[1 1 1] Win Screen
  (`|ExecutionSequence`
    (:`then_0`
      (`self.Get Cubes Amount`)
      (`self.ChangeScoreboardText`))
    (:`then_1`
      (if (`/Game/RollMarker/Blueprints/BP_Brain.areCubesCounted` (`self.BrainRef`))
        (if (== (`self.TotalCubesAmount`) (`self.CurrentMarkedCubesAmount`))
          (`/Engine/EditorBlueprintResources/StandardMacros.DoOnce` false
            (:`Completed`
              (`self.Victory`))))))))

(event `Get Cubes Amount`
  (bind _brainref (`self.BrainRef`))
  ;[1 1 1] Get amount of cubes from Spawner
  (if (`/Game/RollMarker/Blueprints/BP_Brain.areCubesCounted` _brainref)
    (`/Engine/EditorBlueprintResources/StandardMacros.DoOnce` false
      (:`Completed`
        (set `self.TotalCubesAmount` (`/Game/RollMarker/Blueprints/BP_Brain.TotalCubes` _brainref))))))

(event `ChangeScoreboardText`
  (if (`/Game/RollMarker/Blueprints/BP_Brain.areCubesCounted` (`self.BrainRef`))
    (`/Engine/EditorBlueprintResources/StandardMacros.DoOnce` false
      (:`Completed`
        (`/Game/RollMarker/Blueprints/BP_ScoreBoard.Change Score Text` (`self.ScoreboardRef`))))))

(fn `CheckMarked`
  (params (isMarked :type Boolean))
  (bind _currentmarkedcubesamount (`self.CurrentMarkedCubesAmount`))
  (if isMarked
    (`/Engine/EditorBlueprintResources/StandardMacros.IncrementInt` _currentmarkedcubesamount
      (:`  `
        _))
    (else
      (`/Engine/EditorBlueprintResources/StandardMacros.DecrementInt` _currentmarkedcubesamount
        (:`  `
          _))))
  (bind _output_get (set `self.CurrentMarkedCubesAmount` _currentmarkedcubesamount))
  (`/Game/RollMarker/Blueprints/BP_Brain.SetMarkedCubesAmount` (`self.BrainRef`) _output_get)
  (`/Game/RollMarker/Blueprints/BP_ScoreBoard.Change Score Text` (`self.ScoreboardRef`)))

(fn `UserConstructionScript`)

(fn `Victory`
  (bind _returnvalue (`GameplayStatics.GetPlayerController` 0))
  (`GameplayStatics.PlaySound2D` (`self.VictorySound`) 0.2 1.0 0.0 null null)
  (bind _returnvalue_2 (`|GenericCreateObject` "/Game/RollMarker/UI/W_VictoryScreen.W_VictoryScreen_C"))
  (`UserWidget.AddToViewport` _returnvalue_2 0)
  (set `PlayerController.bShowMouseCursor` true _returnvalue)
  (`GameplayStatics.SetGamePaused` true)
  (`WidgetBlueprintLibrary.SetInputMode_UIOnlyEx` _returnvalue null))