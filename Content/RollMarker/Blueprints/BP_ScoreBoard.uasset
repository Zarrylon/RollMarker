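; BP_ScoreBoard is an in-world scoreboard that displays how many cubes are still unmarked.
; On BeginPlay it caches the first BP_Brain actor found in the level as the source of the cube counts.
; Its ChangeScoreText event, not called within this Blueprint, sets the TextRender to the default text plus total minus marked cubes, only once the brain reports the cubes as counted.
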(event `GetBrainRef`
  (bind _outactors (`GameplayStatics.GetAllActorsOfClass` "/Game/RollMarker/Blueprints/BP_Brain.BP_Brain_C"))
  (set `self.Brain Ref` (`|GetArrayItem` _outactors)))

(event `self.ReceiveBeginPlay`
  (`self.GetBrainRef`))

(event `Change Score Text`
  (bind _brain_ref (`self.Brain Ref`))
  ;[1 1 1] Change Scoreboard text
  (if (`/Game/RollMarker/Blueprints/BP_Brain.areCubesCounted` _brain_ref)
    (`TextRenderComponent.K2_SetText` (`self.TextRender`) (`KismetTextLibrary.Conv_StringToText` (`KismetStringLibrary.Concat_StrStr` (`self.DefaultText`) (`KismetStringLibrary.Conv_IntToString` (- (`/Game/RollMarker/Blueprints/BP_Brain.TotalCubes` _brain_ref) (`/Game/RollMarker/Blueprints/BP_Brain.MarkedCubes` _brain_ref))))))))

(fn `UserConstructionScript`)