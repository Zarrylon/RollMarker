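; BP_Spawner fills its Bound volume with target and cleaner cubes when play begins.
; Counts are either preset or, with DoRandomAmount, randomized so cleaners number about half the targets.
; Each cube spawns at a random point inside the bounds with zero rotation.
; It then passes the combined total to the first BP_Brain found in the level and signals that counting is done.
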(event `GetBrainRef`
  ;[1 1 1] References
  (bind _outactors (`GameplayStatics.GetAllActorsOfClass` "/Game/RollMarker/Blueprints/BP_Brain.BP_Brain_C"))
  (set `self.BrainRef` (`|GetArrayItem` _outactors)))

(event `Get Total Amount`
  ;[1 1 1] Get number of cubes
  (bind _output_get (set `self.TotalAmount` (+ (`self.TargetSpawnAmount`) (`self.CleanerSpawnAmount`)))))

(event `self.ReceiveBeginPlay`
  (bind _brainref (`self.BrainRef`))
  ;[1 1 1] Spawning
  (`self.GetBrainRef`)
  (`self.RandomCubeAmount` (`self.DoRandomAmount`))
  (for _ (range 1 (+ (`self.TargetSpawnAmount`) 1))
    (`self.SpawnCube` (`self.TargetClass`)))
  (for _ (range 1 (+ (`self.CleanerSpawnAmount`) 1))
    (`self.SpawnCube` (`self.CleanerClass`)))
  (`self.Get Total Amount`)
  (`/Game/RollMarker/Blueprints/BP_Brain.SetCubesAmount` _brainref (`self.TotalAmount`))
  (`/Game/RollMarker/Blueprints/BP_Brain.DoCubesCounted` _brainref))

(event `RandomCubeAmount`
  (params (doRandom :type Boolean))
  ;[1 1 1] Spawn random amount of cubes.
  ; From 2 to 10 target cubes = n
  ; n/2 or (n/2)+1 cleaner cubes.
  (if doRandom
    (bind _output_get (set `self.TargetSpawnAmount` (`KismetMathLibrary.RandomIntegerInRange` 2 10)))
    (set `self.CleanerSpawnAmount` (+ (`KismetMathLibrary.RandomIntegerInRange` 0 1) (/ _output_get 2)))))

(fn `DoCubesCounted`
  (returns (Success :type Boolean))
  (return false))

(fn `GetTotalCubes`
  (returns (Cubes :type Integer))
  (return (`self.TotalAmount`)))

(fn `SpawnCube`
  (params (CubeClass :type "Actor Class Reference"))
  (locals (CubeType :type "Actor Object Reference" :default "None"))
  (bind (_origin _boxextent) (`KismetSystemLibrary.GetComponentBounds` (`self.Bound`)))
  (`|SpawnActorFromClass` CubeClass (`KismetMathLibrary.MakeTransform` (`KismetMathLibrary.RandomPointInBoundingBox` _origin _boxextent)) "Undefined" "MultiplyWithRoot" null null))

(fn `UserConstructionScript`)